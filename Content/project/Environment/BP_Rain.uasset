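; BP_Rain is a rain zone that fades rain particles and audio in and out as the player character crosses its box collision.
; Entering shows and activates both effects, then plays a timeline that drives audio volume and particle spawn rate from one track.
; Leaving reverses that timeline with a lower spawn-rate scale.
; An IsRain flag, cleared during reverse playback, lets the timeline's finish hide the rain and deactivate the audio.
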(event OnComponentBeginOverlap(BoxCollision)
  (params (OverlappedComponent :type Primitive%20Component%20Object%20Reference) (OtherActor :type Actor%20Object%20Reference) (OtherComp :type Primitive%20Component%20Object%20Reference) (OtherBodyIndex :type Integer) (bFromSweep :type Boolean) (SweepResult :type Hit%20Result%20Structure%20%28by%20ref%29))
  (bind _rain (Variables|Default|GetRain))
  (Utilities|Casting|CastToBP_PlayerCharacter OtherActor)
  (Effects|Components|ParticleSystem|SetFloatParameter _rain "SpawnRate" 1.0)
  (Rendering|SetVisibility _rain true false)
  (Components|Activation|Activate (Variables|Default|GetAudio) true)
  (Variables|Default|SetIsRain true)
  (bind (_direction _newtrack_0) (Timeline|Timeline Play)
    (:Update
      (switch Utilities|FlowControl|Switch|SwitchonETimelineDirection _direction
        (:Forward
          (Audio|Components|Audio|SetVolumeMultiplier (Variables|Default|GetAudio) _newtrack_0 :!class /Script/Engine.AudioComponent)
          (Effects|Components|ParticleSystem|SetFloatParameter (Variables|Default|GetRain) "SpawnRate" (* _newtrack_0 5e+02)))
        (:Backward
          (Variables|Default|SetIsRain false)
          (Audio|Components|Audio|SetVolumeMultiplier (Variables|Default|GetAudio) _newtrack_0 :!class /Script/Engine.AudioComponent)
          (Effects|Components|ParticleSystem|SetFloatParameter (Variables|Default|GetRain) "SpawnRate" (* _newtrack_0 3e+02)))))
    (:Finished
      (if (not (Variables|Default|GetIsRain))
        (Components|Activation|SetActive (Variables|Default|GetAudio) false false)
        (Rendering|SetVisibility (Variables|Default|GetRain) false false)))))

(event OnComponentEndOverlap(BoxCollision)
  (params (OverlappedComponent :type Primitive%20Component%20Object%20Reference) (OtherActor :type Actor%20Object%20Reference) (OtherComp :type Primitive%20Component%20Object%20Reference) (OtherBodyIndex :type Integer))
  (Utilities|Casting|CastToBP_PlayerCharacter OtherActor)
  (bind (_direction _newtrack_0) (Timeline|Timeline Reverse)
    (:Update
      (switch Utilities|FlowControl|Switch|SwitchonETimelineDirection _direction
        (:Forward
          (Audio|Components|Audio|SetVolumeMultiplier (Variables|Default|GetAudio) _newtrack_0 :!class /Script/Engine.AudioComponent)
          (Effects|Components|ParticleSystem|SetFloatParameter (Variables|Default|GetRain) "SpawnRate" (* _newtrack_0 5e+02)))
        (:Backward
          (Variables|Default|SetIsRain false)
          (Audio|Components|Audio|SetVolumeMultiplier (Variables|Default|GetAudio) _newtrack_0 :!class /Script/Engine.AudioComponent)
          (Effects|Components|ParticleSystem|SetFloatParameter (Variables|Default|GetRain) "SpawnRate" (* _newtrack_0 3e+02)))))
    (:Finished
      (if (not (Variables|Default|GetIsRain))
        (Components|Activation|SetActive (Variables|Default|GetAudio) false false)
        (Rendering|SetVisibility (Variables|Default|GetRain) false false)))))

(fn ConstructionScript)